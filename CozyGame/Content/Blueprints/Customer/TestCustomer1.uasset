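; Customer actor that requests a random drink type and shows it in a widget while the player character is within its sphere collider.
; Overlapping a drink destroys it and compares the index of its highest flavor attribute to the wanted type, so attribute order must match the enum.
; A match plays a happy sound, has CustomerSpawner actors spawn a customer at its transform and destroys itself; a mismatch plays a sad sound.
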(event `self.ReceiveBeginPlay`
  ;[1 1 1] Random requested drink
  (bind _output_get (set `self.DrinkTypeWanted` (cast `/Game/Blueprints/Enum_DrinkType` (`KismetMathLibrary.Conv_IntToByte` (`KismetMathLibrary.RandomIntegerInRange` 0 9)))))
  (bind _returnvalue (`|GetEnumeratorNameAsString` _output_get))
  (`KismetSystemLibrary.PrintString` (`KismetStringLibrary.Concat_StrStr` "Customer wants: " _returnvalue))
  (bind _aswbp_requested_drink (cast `/Game/UI/WBP_RequestedDrink` (`WidgetComponent.GetUserWidgetObject` (`self.RequestedDrinkWidget`))))
  (`/Game/UI/WBP_RequestedDrink.Update` _aswbp_requested_drink _returnvalue))

(event `self.Drink Collider.OnComponentBeginOverlap`
  (params (OverlappedComponent :type "PrimitiveComponent Object Reference") (OtherActor :type "Actor Object Reference") (OtherComp :type "PrimitiveComponent Object Reference") (OtherBodyIndex :type Integer) (bFromSweep :type Boolean) (SweepResult :type "HitResult Structure (by ref)"))
  (bind _returnvalue (`self.GetComponentByClass` OtherActor "/Game/Blueprints/BP_Drink.BP_Drink_C"))
  (`/Engine/EditorBlueprintResources/StandardMacros.IsValid` _returnvalue
    (:`Is Valid`
      ;[1 1 1] Give Drink Function Here if Valid
      (bind _isequal (`self.Compare Drinks` OtherActor _returnvalue))
      (`KismetSystemLibrary.PrintString` (`KismetStringLibrary.Concat_StrStr` "Received correct drink: " (`KismetStringLibrary.Conv_BoolToString` _isequal)))
      ;[1 1 1] Play sound based on whether or not received drink matches requested drink
      (if _isequal
        (`GameplayStatics.PlaySoundAtLocation` "/Game/Sounds/SoundEffects/customer_happy_sound.customer_happy_sound" (`self.K2_GetActorLocation`) (struct) 1.0 1.0 0.0 null null null null)
        (bind _outactors (`GameplayStatics.GetAllActorsOfClass` "/Game/Blueprints/Customer/CustomerSpawner.CustomerSpawner_C"))
        (for _array_element _outactors
          (`/Game/Blueprints/Customer/CustomerSpawner.SpawnCustomer` _array_element (`self.K2_GetActorLocation`) (`self.K2_GetActorRotation`))
          (`self.K2_DestroyActor`))
        (else
          (`GameplayStatics.PlaySoundAtLocation` "/Game/Sounds/SoundEffects/customer_sad_sound.customer_sad_sound" (`self.K2_GetActorLocation`) (struct) 1.0 1.0 0.0 null null null null))))
    (:`Is Not Valid`
      (`KismetSystemLibrary.PrintString` "No valid drink for customer" false))))

(event `self.SphereCollider.OnComponentBeginOverlap`
  (params (OverlappedComponent :type "PrimitiveComponent Object Reference") (OtherActor :type "Actor Object Reference") (OtherComp :type "PrimitiveComponent Object Reference") (OtherBodyIndex :type Integer) (bFromSweep :type Boolean) (SweepResult :type "HitResult Structure (by ref)"))
  (cast `/Game/ThirdPerson/Blueprints/BP_ThirdPersonCharacter` OtherActor)
  (`SceneComponent.SetVisibility` (`self.RequestedDrinkWidget`) true false))

(event `self.SphereCollider.OnComponentEndOverlap`
  (params (OverlappedComponent :type "PrimitiveComponent Object Reference") (OtherActor :type "Actor Object Reference") (OtherComp :type "PrimitiveComponent Object Reference") (OtherBodyIndex :type Integer))
  (cast `/Game/ThirdPerson/Blueprints/BP_ThirdPersonCharacter` OtherActor)
  (`SceneComponent.SetVisibility` (`self.RequestedDrinkWidget`) false false))

(fn `Compare Drinks`
  (params (GivenDrinkActor :type "Actor Object Reference") (GivenDrinkComponent :type "/Game/Blueprints/BP_Drink Object Reference"))
  (returns (isEqual :type Boolean))
  (locals (attributeArray :type "Array of Integer"))
  (bind _attributearray (`local.attributeArray`))
  (bind (_sweet _bitter _sour _nutty _vegetative _fermented _musty _chemical _papery _fruity) (break `/Game/Blueprints/F_Attributes` (`.Attributes_10_41159F3D4470EF93A5A095B0CA622700` (break `/Game/Blueprints/F_Drink` (`/Game/Blueprints/BP_Drink.DrinkData` GivenDrinkComponent)))))
  ;[1 1 1] Create attribute array
  (`KismetArrayLibrary.Array_Add` _attributearray _sweet)
  (`KismetArrayLibrary.Array_Add` _attributearray _bitter)
  (`KismetArrayLibrary.Array_Add` _attributearray _sour)
  (`KismetArrayLibrary.Array_Add` _attributearray _nutty)
  (`KismetArrayLibrary.Array_Add` _attributearray _vegetative)
  (`KismetArrayLibrary.Array_Add` _attributearray _fermented)
  (`KismetArrayLibrary.Array_Add` _attributearray _musty)
  (`KismetArrayLibrary.Array_Add` _attributearray _chemical)
  (`KismetArrayLibrary.Array_Add` _attributearray _papery)
  (`KismetArrayLibrary.Array_Add` _attributearray _fruity)
  (`self.K2_DestroyActor` GivenDrinkActor)
  (return (== (`KismetMathLibrary.Conv_ByteToInt` (`self.DrinkTypeWanted`)) (`KismetMathLibrary.MaxOfIntArray` (`local.attributeArray`)))))

(fn `UserConstructionScript`)