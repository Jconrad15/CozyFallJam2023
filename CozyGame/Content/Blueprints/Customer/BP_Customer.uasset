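; BP_Customer is a customer that receives drinks by being hit with them and judges whether they match its wanted attributes.
; On Hit, it looks for a BP_Drink component on the other actor, then plays a happy or sad sound from the CompareDrinks result.
; CompareDrinks compares only the summed Sweet, Bitter and Sour totals, then destroys the drink actor.
; BeginPlay is empty, with random drink selection noted only in a comment.
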(event `self.ReceiveBeginPlay`
  ;[1 1 1] set wanted drink to random from array
)

(event `self.ReceiveHit`
  (params (MyComp :type "PrimitiveComponent Object Reference") (Other :type "Actor Object Reference") (OtherComp :type "PrimitiveComponent Object Reference") (bSelfMoved :type Boolean) (HitLocation :type "Vector Structure") (HitNormal :type "Vector Structure") (NormalImpulse :type "Vector Structure") (Hit :type "HitResult Structure (by ref)"))
  (bind _returnvalue (`self.GetComponentByClass` Other "/Game/Blueprints/BP_Drink.BP_Drink_C"))
  (`/Engine/EditorBlueprintResources/StandardMacros.IsValid` _returnvalue
    (:`Is Valid`
      ;[1 1 1] Give Drink Function Here if Valid
      (bind _isequal (`self.Compare Drinks` Other _returnvalue))
      (if _isequal
        (`GameplayStatics.PlaySoundAtLocation` "/Game/Sounds/SoundEffects/customer_happy_sound.customer_happy_sound" (`self.K2_GetActorLocation`) (struct) 1.0 1.0 0.0 null null null null)
        (else
          (`GameplayStatics.PlaySoundAtLocation` "/Game/Sounds/SoundEffects/customer_sad_sound.customer_sad_sound" (`self.K2_GetActorLocation`) (struct) 1.0 1.0 0.0 null null null null))))
    (:`Is Not Valid`
      (`KismetSystemLibrary.PrintString` "No valid drink for customer"))))

(fn `Compare Drinks`
  (params (GivenDrinkActor :type "Actor Object Reference") (GivenDrinkComponent :type "/Game/Blueprints/BP_Drink Object Reference"))
  (returns (isEqual :type Boolean))
  (locals (tempisEqual :type Boolean))
  (bind _drinkdata (`/Game/Blueprints/BP_Drink.DrinkData` GivenDrinkComponent))
  (bind (_attributeswanted_sweet _attributeswanted_bitter _attributeswanted_sour) (break `/Game/Blueprints/F_Attributes` (`self.AttributesWanted`)))
  (`KismetSystemLibrary.PrintString` (`KismetStringLibrary.Conv_IntToString` (break `/Game/Blueprints/F_Attributes` (`.Attributes_10_41159F3D4470EF93A5A095B0CA622700` (break `/Game/Blueprints/F_Drink` _drinkdata)))))
  (`KismetSystemLibrary.PrintString` (`KismetStringLibrary.Conv_IntToString` _attributeswanted_sweet))
  (bind _output_get (set `local.tempisEqual` (== (+ (break `/Game/Blueprints/F_Attributes` (`.Attributes_10_41159F3D4470EF93A5A095B0CA622700` (break `/Game/Blueprints/F_Drink` _drinkdata))) (`.Bitter_4_A7B1FBC343EA7EDA6E2721B57F4117BE` (break `/Game/Blueprints/F_Attributes` (`.Attributes_10_41159F3D4470EF93A5A095B0CA622700` (break `/Game/Blueprints/F_Drink` _drinkdata)))) (`.Sour_6_E7AB63704499F7DCE791B19D813D4B6E` (break `/Game/Blueprints/F_Attributes` (`.Attributes_10_41159F3D4470EF93A5A095B0CA622700` (break `/Game/Blueprints/F_Drink` _drinkdata))))) (+ _attributeswanted_sweet _attributeswanted_bitter _attributeswanted_sour))))
  (`self.K2_DestroyActor` GivenDrinkActor)
  (return _output_get))

(fn `UserConstructionScript`)