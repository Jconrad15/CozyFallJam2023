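; Mixer actor that absorbs ingredient actors that hit it and turns the blend into a drink.
; Hits from actors with a BP_Ingredient component add their Sweet, Bitter and Sour values to a running blend, then destroy the ingredient.
; CreateDrink, not called within this Blueprint, spawns a TestDrink beside the mixer if ingredients exist, sets its data, picks its mesh by the strongest attribute, and resets the mixer.
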(event `self.ReceiveBeginPlay`
  (set `self.CurrentBlendAttributes` (make `/Game/Blueprints/F_Attributes` 0)))

(event `self.ReceiveHit`
  (params (MyComp :type "PrimitiveComponent Object Reference") (Other :type "Actor Object Reference") (OtherComp :type "PrimitiveComponent Object Reference") (bSelfMoved :type Boolean) (HitLocation :type "Vector Structure") (HitNormal :type "Vector Structure") (NormalImpulse :type "Vector Structure") (Hit :type "HitResult Structure (by ref)"))
  (bind _returnvalue (`self.GetComponentByClass` Other "/Game/Blueprints/BP_Ingredient.BP_Ingredient_C"))
  (`/Engine/EditorBlueprintResources/StandardMacros.IsValid` _returnvalue
    (:`Is Valid`
      (`self.AddIngredient` Other _returnvalue)
      (`GameplayStatics.PlaySoundAtLocation` "/Game/Sounds/SoundEffects/drop_drink_sound.drop_drink_sound" (`self.K2_GetActorLocation`) (struct) 1.0 1.0 0.0 null null null null))
    (:`Is Not Valid`
      (`KismetSystemLibrary.PrintString` "Not valid ingredient for mixer" false true (struct :`R` 1.0 :`G` 0.332784 :`B` 0.322837 :`A` 1.0) 1.0))))

(fn `AddIngredient`
  (params (IngredientActor :type "Actor Object Reference") (IngredientComponent :type "/Game/Blueprints/BP_Ingredient Object Reference"))
  (bind (_ingredientdata_name _ingredientdata_description _ingredientdata_attributes) (break `/Game/Blueprints/F_Ingredient` (`/Game/Blueprints/BP_Ingredient.IngredientData` IngredientComponent)))
  (bind (_currentblendattributes_sweet _currentblendattributes_bitter _currentblendattributes_sour) (break `/Game/Blueprints/F_Attributes` (`self.CurrentBlendAttributes`)))
  (bind (_sweet _bitter _sour) (break `/Game/Blueprints/F_Attributes` _ingredientdata_attributes))
  (set `self.CurrentBlendAttributes` (make `/Game/Blueprints/F_Attributes` (+ _currentblendattributes_sweet _sweet) (+ _currentblendattributes_bitter _bitter) (+ _currentblendattributes_sour _sour)))
  (`/Engine/EditorBlueprintResources/StandardMacros.IncrementInt` (`self.CurrentIngredientCount`)
    (:`  `
      (`self.K2_DestroyActor` IngredientActor))))

(fn `CreateDrink`
  (bind (_drink _makedrink _mesh) (`self.DetermineOutputDrink`))
  (if _makedrink
    ;[1 1 1] Spawn Drink
    (bind _returnvalue (`|SpawnActorFromClass` "/Game/Blueprints/Drinks/TestDrink.TestDrink_C" (`KismetMathLibrary.MakeTransform` (+ (`self.K2_GetActorLocation`) (60.0 0.0 0.0))) "Undefined" "MultiplyWithRoot" null null))
    ;[1 1 1] Set created drink attributes
    (set `/Game/Blueprints/BP_Drink.DrinkData` _drink (`self.GetComponentByClass` _returnvalue "/Game/Blueprints/BP_Drink.BP_Drink_C"))
    ;[1 1 1] Set create drink mesh
    (`StaticMeshComponent.SetStaticMesh` (`/Game/Blueprints/Drinks/TestDrink.Model` _returnvalue) _mesh)
    (set `self.CurrentIngredientCount` 0) ; Used up all ingredients
    ;[1 1 1] Play Create drink sound
    (`GameplayStatics.PlaySoundAtLocation` "/Game/Sounds/SoundEffects/Bubble.Bubble" (`self.K2_GetActorLocation` _returnvalue) (struct) 1.0 1.0 0.0 null null null null)
    (else
      (`KismetSystemLibrary.PrintString` "Don't make drink"))))

(fn `DetermineOutputDrink`
  (returns (Drink :type "/Game/Blueprints/F_Drink Structure") (MakeDrink :type Boolean) (Mesh :type "StaticMesh Object Reference"))
  (locals (DrinkAttributes :type "/Game/Blueprints/F_Attributes Structure") (DrinkMeshIndex :type Integer) (AttributeArray :type "Array of Integer"))
  (bind (_drinkattributes_sweet _drinkattributes_bitter _drinkattributes_sour) (break `/Game/Blueprints/F_Attributes` (`local.DrinkAttributes`)))
  ;[1 1 1] Check if there are any current ingredients
  (if (== (`self.CurrentIngredientCount`) 0)
    (return (make `/Game/Blueprints/F_Drink` "None") false null)
    (else
      (bind _output_get (set `local.DrinkAttributes` (`self.CurrentBlendAttributes`)))
      (set `self.CurrentBlendAttributes` (struct)) ; Set current attributes to zero
      ;[1 1 1] Create array of attribute values
      (`KismetArrayLibrary.Array_Add` (`local.AttributeArray`) _drinkattributes_sweet)
      (`KismetArrayLibrary.Array_Add` (`local.AttributeArray`) _drinkattributes_bitter)
      (`KismetArrayLibrary.Array_Add` (`local.AttributeArray`) _drinkattributes_sour)
      (return (make `/Game/Blueprints/F_Drink` "Test drink" _output_get) true (select `int` (`KismetMathLibrary.MaxOfIntArray` (`local.AttributeArray`)) :`0` "/Game/Assets/Drinks/drink_7_sweet_folder/drink7_sweet.drink7_sweet" :`1` "/Game/Assets/Drinks/drink_8_bitter_folder/drink8_bitter.drink8_bitter" :`2` "/Game/Assets/Drinks/drink_9_sour_folder/drink9_sour.drink9_sour" :!type "StaticMesh Object Reference")))))

(fn `UserConstructionScript`)