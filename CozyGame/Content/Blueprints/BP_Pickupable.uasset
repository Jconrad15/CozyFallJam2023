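; BP_Pickupable is a component that lets its owning actor be picked up and dropped by the player.
; Pickup and TryDrop flip IsPickedUp and toggle physics simulation on all the owner's primitive components, with TryDrop returning whether it dropped.
; While held, Tick moves the owner to the third-person character's HeldItemLocation each frame, changing only location.
; Debug prints trace each action, and an unconnected SetWorldTransform node remains unused.
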(event `self.ReceiveBeginPlay`
  (set `self.Owner` (`self.GetOwner`)))

(event `self.ReceiveTick`
  (params (DeltaSeconds :type "Float (single-precision)"))
  (if (`self.IsPickedUp`)
    (bind _asbp_third_person_character (cast `/Game/ThirdPerson/Blueprints/BP_ThirdPersonCharacter` (`GameplayStatics.GetPlayerCharacter` 0)))
    (`Actor.K2_SetActorLocation` (`self.GetOwner`) (`/Game/ThirdPerson/Blueprints/BP_ThirdPersonCharacter.HeldItemLocation` _asbp_third_person_character) false false)))

(fn `Pickup`
  (`KismetSystemLibrary.PrintString` "Pick up")
  (if (`self.IsPickedUp`)
    (`KismetSystemLibrary.PrintString` "Errror")
    (else
      (`self.TogglePhysics` false)
      (set `self.IsPickedUp` true))))

(fn `TogglePhysics`
  (params (TurnOn :type Boolean))
  (for _array_element (`Actor.K2_GetComponentsByClass` (`self.Owner`) "/Script/Engine.PrimitiveComponent")
    (`PrimitiveComponent.SetSimulatePhysics` _array_element TurnOn)
    (`KismetSystemLibrary.PrintString` (`KismetStringLibrary.Concat_StrStr` "Physics is on: " (`KismetStringLibrary.Conv_BoolToString` TurnOn)))))

(fn `Try Drop`
  (returns (wasDropped :type Boolean))
  (if (`self.IsPickedUp`)
    (set `self.IsPickedUp` false)
    (`self.TogglePhysics` true)
    (`KismetSystemLibrary.PrintString` "Dropped" true true (struct :`R` 0.167905 :`G` 1.0 :`B` 0.227356 :`A` 1.0))
    (return true)
    (else
      (return false))))